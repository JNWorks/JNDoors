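; BP_PhysicDoor is a door that swings as a simulated physics body, hinged to its frame by an angle-limited constraint configured at BeginPlay.
; Open/close events apply an impulse, choosing push direction from the current yaw or supplied opening side.
; Tick replays the movement sound on positive angular velocity, throttled by a resettable DoOnce.
; Authority-triggered snap-shut with a closing sound near zero yaw is flag-gated and marked unfinished.
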(event `self.ReceiveBeginPlay`
  (bind _returnvalue (`self.GetComponentByClass` (`self.Door`) "/Script/Engine.StaticMeshComponent"))
  (`parent.ReceiveBeginPlay`)
  (set `self.MaxOpenAngle` (* (`self.MaxOpenAngle`) 2.0))
  (`PrimitiveComponent.SetSimulatePhysics` _returnvalue true)
  (`PrimitiveComponent.SetCollisionProfileName` _returnvalue "PhysicsActor" true)
  (`PhysicsConstraintComponent.SetAngularSwing1Limit` (`self.PhysicsConstraint`) "ACM_Limited" (/ (`self.MaxOpenAngle`) (`KismetMathLibrary.SelectFloat` 1.0 2.0 (`self.OpenToBothSides`))))
  (`PhysicsConstraintComponent.SetConstrainedComponents` (`self.PhysicsConstraint`) (`self.Frame`) "None" (`self.GetDoorModel`) "None")
  (`KismetSystemLibrary.Delay` 2.0)
  (`self.EnableMovingSoundMulticast`))

(event `self.OpenCloseMulticast`
  (params (OpeningSide :type Boolean))
  (bind _returnvalue (`self.GetDoorModel`))
  (bind _pushforce (`self.PushForce`))
  (bind (_relativerotation_roll _relativerotation_pitch _relativerotation_yaw) (`KismetMathLibrary.BreakRotator` (`SceneComponent.RelativeRotation` _returnvalue)))
  (bind (_relativerotation_roll_2 _relativerotation_pitch_2 _relativerotation_yaw_2) (`KismetMathLibrary.BreakRotator` (`SceneComponent.RelativeRotation` _returnvalue)))
  (`AudioComponent.Play` (`self.DoorMoving`) 0.0)
  (`/Game/Doors/SA_DoorModel.ApplyImpulse` (`self.Door`) (* (`SceneComponent.GetForwardVector` (`self.GetDoorModel`)) (`KismetMathLibrary.SelectFloat` (* _pushforce -1.0) _pushforce (select `bool` (> (`KismetMathLibrary.Abs` _relativerotation_yaw) (/ (`self.MaxOpenAngle`) 4.0)) :`false` OpeningSide :`true` (> _relativerotation_yaw_2 (/ (`self.MaxOpenAngle`) 4.0))))) (`SceneComponent.K2_GetComponentLocation` (`self.WithoutHandle`))))

(event `self.ReceiveTick`
  (params (DeltaSeconds :type "Float (single-precision)"))
  (bind (_returnvalue_x _returnvalue_y _returnvalue_z) (`KismetMathLibrary.BreakVector` (`PrimitiveComponent.GetPhysicsAngularVelocityInDegrees` (`self.GetDoorModel`) "None")))
  (bind (_relativerotation_roll _relativerotation_pitch _relativerotation_yaw) (`KismetMathLibrary.BreakRotator` (`SceneComponent.RelativeRotation` (`self.GetDoorModel`))))
  (`parent.ReceiveTick` 0.0)
  (`|ExecutionSequence`
    (:`then_0`
      (if (> _returnvalue_z 0.0)
        (`/Engine/EditorBlueprintResources/StandardMacros.DoOnce` true :!label _label
          (:`Completed`
            (`AudioComponent.Play` (`self.DoorMoving`) 0.3)
            (`KismetSystemLibrary.Delay` 0.5)
            (goto _label :!via `Reset`)))))
    (:`then_1`
      ;[1 1 1] To be implemented (close door sound)
      (if (and (`KismetMathLibrary.NearlyEqual_FloatFloat` _relativerotation_yaw 0.0 10.0) (`self.EnableClosePhysicDoor?(TODO)`))
        (`/Engine/EditorBlueprintResources/StandardMacros.DoOnce` true :!label _label_2
          (:`Completed`
            (`/Engine/EditorBlueprintResources/ActorMacros.Switch Has Authority`
              (:`Authority`
                (`self.ClosePhysicDoorMulticast`)))))
        (else
          (goto _label_2 :!via `Reset`))))))

(event `EnableMovingSoundMulticast`
  (goto _label :!via `Reset`))

(event `ClosePhysicDoorMulticast`
  (bind _returnvalue (`self.GetDoorModel`))
  ;[1 1 1] To be implemented (close door sound)
  (`SceneComponent.K2_SetRelativeRotation` :`self` _returnvalue :`bTeleport` true)
  (`PrimitiveComponent.SetAllPhysicsAngularVelocityInDegrees` _returnvalue (0.0 0.0 0.0) false)
  (`AudioComponent.Play` (`self.Closing`) 0.0))

(fn `GetDoorModel`
  (returns (ReturnValue :type "StaticMeshComponent Object Reference"))
  (return (`self.GetComponentByClass` (`ChildActorComponent.ChildActor` (`self.DoorModel`)) "/Script/Engine.StaticMeshComponent")))

(fn `UserConstructionScript`
  (`parent.UserConstructionScript`))