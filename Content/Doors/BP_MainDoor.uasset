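; Interactive swinging door that players open and close with E, with sounds and an on-screen prompt.
; A range volume tracks the local player and registers with AC_CanOpenDoor, while a camera trace against the handle or door gates prompt and input.
; OpenCloseMulticast runs a curve-driven timeline rotating the child-actor model, optionally away from the player's side.
; Collision loosens during movement; an overlap halts the swing and restores blocking.
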(event `self.ReceiveBeginPlay`
  (bind _alphacurve (`self.AlphaCurve`))
  (bind (_mintime _maxtime) (`CurveBase.GetTimeRange` _alphacurve))
  (`|ExecutionSequence`
    (:`then_0`
      ;[0.5052 0.5052 0.5052] Handle Setup
      (if (`self.UseHandle`)
        (`PrimitiveComponent.SetCollisionResponseToChannel` (`self.WithHandle`) "ECC_Visibility" "ECR_Block")))
    (:`then_1`
      ;[1 1 1] Attach handles to the door
      (bind _assa_door_model (cast `/Game/Doors/SA_DoorModel` (`ChildActorComponent.ChildActor` (`self.DoorModel`))))
      (bind _output_get (set `self.Door` _assa_door_model))
      (bind _returnvalue (`self.GetComponentByClass` _output_get "/Script/Engine.StaticMeshComponent"))
      (`SceneComponent.K2_AttachToComponent` (`self.WithoutHandle`) _returnvalue "None" "KeepRelative" "KeepRelative" "KeepRelative" false)
      (`SceneComponent.K2_AttachToComponent` _returnvalue (`self.Frame`) "None" "KeepWorld" "KeepWorld" "KeepWorld" true))
    (:`then_2`
      (`AudioComponent.SetSound` (`self.Closing`) (`self.ClosingSound`))
      (`AudioComponent.SetSound` (`self.DoorMoving`) (`self.MovingSound`))
      (`AudioComponent.SetSound` (`self.Opening`) (`self.OpenSound`))
      (set `self.DoorResponse` (select `bool` (`self.CharacterBlockDoor`) :`false` (enumliteral `ECollisionResponse` "ECR_Ignore") :`true` (enumliteral `ECollisionResponse` "ECR_Overlap")))
      (set `self.DrawDebugTracing` (select `bool` (`self.ShowAimingDebug`) :`false` (enumliteral `EDrawDebugTrace` "None") :`true` (enumliteral `EDrawDebugTrace` "ForDuration")))
      (bind _returnvalue_2 (`|CreateWidget` "/Game/Doors/Widget_PressToOpen.Widget_PressToOpen_C" (`GameplayStatics.GetPlayerController` 0)))
      (`UserWidget.AddToViewport` _returnvalue_2 0)
      (set `self.PressToOpenWidget` _returnvalue_2)
      (`self.HideUI`)
      (`/Engine/EditorBlueprintResources/StandardMacros.IsValid` (`self.AlphaCurve`)
        (:`Is Valid`
          (`TimelineComponent.SetFloatCurve` (`self.OpenCloseTimeLine`) _alphacurve "Alpha")
          (`TimelineComponent.SetTimelineLength` (`self.OpenCloseTimeLine`) (+ _maxtime 0.05))
          (`AudioComponent.SetPitchMultiplier` (`self.DoorMoving`) (`KismetMathLibrary.FClamp` (/ 1.0 _maxtime) 0.8 1.2)))))))

(event `OpenCloseMulticast`
  (params (OpeningSide :type Boolean))
  (bind _openingsoundduration (`self.OpeningSoundDuration`))
  (bind _closing (`self.Closing`))
  (bind _opening (`self.Opening`))
  (bind _closingsoundduration (`self.ClosingSoundDuration`))
  (bind _returnvalue (select `bool` (`self.OpenToBothSides`) :`false` (`self.InvertOpenSide (IfBothSidesDisabled)`) :`true` (select `bool` (`self.Opened?`) :`false` OpeningSide :`true` (`self.OpenedSide`))))
  (if (< (stale _alpha) 0.5)
    (bind (_direction _alpha) (`Timeline|OpenCloseTimeline` :!label _label)
      (:`Update`
        (bind _returnvalue_2 (< _alpha 0.05))
        (if _returnvalue_2
          (`|ExecutionSequence`
            (:`then_0`
              (switch `ETimelineDirection` _direction
                (:`Forward`
                  (`|ExecutionSequence`
                    (:`then_0`
                      (`/Engine/EditorBlueprintResources/StandardMacros.DoOnce` false :!label _label_2
                        (:`Completed`
                          (`AudioComponent.Play` _opening (`self.OpeningSoundStartTime`))
                          (if (> _openingsoundduration 0.0)
                            (`AudioComponent.StopDelayed` _opening _openingsoundduration)))))
                    (:`then_1`
                      (goto _label_3 :!via `Reset`))))
                (:`Backward`
                  (`|ExecutionSequence`
                    (:`then_0`
                      (goto _label_2 :!via `Reset`))
                    (:`then_1`
                      (`/Engine/EditorBlueprintResources/StandardMacros.DoOnce` true :!label _label_3
                        (:`Completed`
                          (`AudioComponent.Play` _closing (`self.ClosingSoundStartTime`))
                          (if (> _closingsoundduration 0.0)
                            (`AudioComponent.StopDelayed` _closing _closingsoundduration)))))))))
            (:`then_1`
              (set `self.OpenedSide` _returnvalue :!label _label_4)
              (`|ExecutionSequence`
                (:`then_0`
                  (`/Engine/EditorBlueprintResources/StandardMacros.DoOnce` false :!label _label_5
                    (:`Completed`
                      (`AudioComponent.Play` (`self.DoorMoving`) (`self.MovingSoundStartTime`))
                      (`KismetSystemLibrary.Delay` (`self.MovingSoundDuration(Needed)`))
                      (goto _label_5 :!via `Reset`))))
                (:`then_1`
                  (`/Game/Doors/SA_DoorModel.RotateDoor` (`self.Door`) (* _alpha (`self.MaxOpenAngle`) (`KismetMathLibrary.SelectFloat` -1.0 1.0 _returnvalue)))
                  (`/Engine/EditorBlueprintResources/StandardMacros.DoOnce` false :!label _label_6
                    (:`Completed`
                      (`self.SetCollision` (`self.WithoutHandle`) (`self.DoorResponse`))))))))
          (else
            (goto _label_4))))
      (:`Finished`
        (set `self.Opened?` (not _returnvalue_2))
        (`|ExecutionSequence`
          (:`then_1`
            (`AudioComponent.Stop` (`self.DoorMoving`) :!label _label_7)
            (`|ExecutionSequence`
              (:`then_0`
                (goto _label_6 :!via `Reset`))
              (:`then_1`
                (`self.SetCollision` (`self.WithoutHandle`) "ECR_Block")))))))
    (else
      (goto _label :!via `Reverse`))))

(event `self.WithoutHandle.OnComponentBeginOverlap`
  (params (OverlappedComponent :type "PrimitiveComponent Object Reference") (OtherActor :type "Actor Object Reference") (OtherComp :type "PrimitiveComponent Object Reference") (OtherBodyIndex :type Integer) (bFromSweep :type Boolean) (SweepResult :type "HitResult Structure (by ref)"))
  (`|ExecutionSequence`
    (:`then_0`
      (goto _label :!via `Stop`))
    (:`then_1`
      (goto _label_7))))

(event `Key|E`
  (params (Key :type "Key Structure"))
  (:`Pressed`
    (`self.IsAimingTheDoor`
      (:`CanOpen`
        (`self.OpenCloseMulticast` (`self.GetIsOnTheFront`))))))

(event `self.ReceiveTick`
  (params (DeltaSeconds :type "Float (single-precision)"))
  (bind _textrender (`self.TextRender`))
  (bind _canopentxt (`/Game/Doors/Widget_PressToOpen.CanOpenTXT` (`self.PressToOpenWidget`)))
  (bind (_returnvalue_roll _returnvalue_pitch _returnvalue_yaw) (`KismetMathLibrary.BreakRotator` (`KismetMathLibrary.FindLookAtRotation` (`SceneComponent.K2_GetComponentLocation` _textrender) (`self.K2_GetActorLocation` (`GameplayStatics.GetPlayerPawn` 0)))))
  (`|ExecutionSequence`
    (:`then_0`
      (`KismetSystemLibrary.Delay` 0.3)
      (if (`self.InRange?`)
        (`self.IsAimingTheDoor`
          (:`CanOpen`
            (`|ExecutionSequence`
              (:`then_0`
                (`Widget.SetVisibility` _canopentxt "Visible")
                (set `self.CanBeOpened` true)
                (`KismetSystemLibrary.RetriggerableDelay` 0.35)
                (`Widget.SetVisibility` _canopentxt "Hidden"))
              (:`then_1`
                (`|ExecutionSequence` :!label _label_8
                  (:`then_0`
                    (`/Engine/EditorBlueprintResources/StandardMacros.DoOnce` false :!label _label_9
                      (:`Completed`
                        (`self.ShowUI`))))
                  (:`then_1`
                    (goto _label_10 :!via `Reset`))))))
          (:`LookingAtDoor`
            (set `self.CanBeOpened` false)
            (goto _label_8))
          (:`False`
            (`|ExecutionSequence`
              (:`then_0`
                (goto _label_9 :!via `Reset`))
              (:`then_1`
                (`/Engine/EditorBlueprintResources/StandardMacros.DoOnce` true :!label _label_10
                  (:`Completed`
                    (`self.HideUI`)
                    (set `self.CanBeOpened` false)))))))
        (else
          (goto _label_9 :!via `Reset`))))
    (:`then_1`
      (if (not (`self.HideText`))
        (`SceneComponent.K2_SetWorldRotation` _textrender (`KismetMathLibrary.MakeRotator` 0.0 0.0 _returnvalue_yaw) false false)))))

(event `ShowUI`
  (`Widget.SetVisibility` (`self.PressToOpenWidget`) "Visible"))

(event `HideUI`
  (`Widget.SetVisibility` (`self.PressToOpenWidget`) "Hidden"))

(event `self.InRange.OnComponentBeginOverlap`
  (params (OverlappedComponent :type "PrimitiveComponent Object Reference") (OtherActor :type "Actor Object Reference") (OtherComp :type "PrimitiveComponent Object Reference") (OtherBodyIndex :type Integer) (bFromSweep :type Boolean) (SweepResult :type "HitResult Structure (by ref)"))
  (bind _returnvalue (`self.GetComponentByClass` OtherActor "/Game/Doors/AC_CanOpenDoor.AC_CanOpenDoor_C"))
  (bind _aspawn (cast `Pawn` OtherActor))
  (bind _asplayer_controller (cast `PlayerController` (`Pawn.GetController` _aspawn)))
  (if (== _asplayer_controller (`GameplayStatics.GetPlayerController` 0))
    (if (`self.UseDoorSystemToOpen (SinglePlayerOnly)`)
      (`self.EnableInput` _asplayer_controller))
    (set `self.InRange?` true)
    (`/Engine/EditorBlueprintResources/StandardMacros.IsValid` _returnvalue
      (:`Is Valid`
        (set `/Game/Doors/AC_CanOpenDoor.Door` self _returnvalue)))))

(event `self.InRange.OnComponentEndOverlap`
  (params (OverlappedComponent :type "PrimitiveComponent Object Reference") (OtherActor :type "Actor Object Reference") (OtherComp :type "PrimitiveComponent Object Reference") (OtherBodyIndex :type Integer))
  (bind _returnvalue (`self.GetComponentByClass` "/Game/Doors/AC_CanOpenDoor.AC_CanOpenDoor_C"))
  (bind _aspawn (cast `Pawn` OtherActor))
  (bind _asplayer_controller (cast `PlayerController` (`Pawn.GetController` _aspawn)))
  (if (== _asplayer_controller (`GameplayStatics.GetPlayerController` 0))
    (if (`self.UseDoorSystemToOpen (SinglePlayerOnly)`)
      (`self.DisableInput` _asplayer_controller))
    (set `self.InRange?` false)
    (`self.HideUI`)
    (`/Engine/EditorBlueprintResources/StandardMacros.IsValid` _returnvalue
      (:`Is Valid`
        (if (== self (`/Game/Doors/AC_CanOpenDoor.Door` _returnvalue))
          (set `/Game/Doors/AC_CanOpenDoor.Door` null _returnvalue))))))

(fn `GetIsOnTheFront`
  (returns (ReturnValue :type Boolean))
  (return (!= (`KismetArrayLibrary.Array_Find` (`PrimitiveComponent.GetOverlappingActors` (`self.FrontSide`) "/Script/Engine.Pawn") (`GameplayStatics.GetPlayerPawn` 0)) -1)))

(fn `SetCollision`
  (params (Collision :type "BoxComponent Object Reference") (NewResponse :type "ECollisionResponse Enum" :default "ECR_Ignore"))
  (`PrimitiveComponent.SetCollisionResponseToChannel` Collision "ECC_WorldDynamic" NewResponse)
  (`PrimitiveComponent.SetCollisionResponseToChannel` Collision "ECC_Pawn" NewResponse)
  (`PrimitiveComponent.SetCollisionResponseToChannel` Collision "ECC_PhysicsBody" NewResponse)
  (`PrimitiveComponent.SetCollisionResponseToChannel` Collision "ECC_Vehicle" NewResponse)
  (if (`|EnumInequality` "ECR_Overlap" NewResponse)
    (`PrimitiveComponent.SetCollisionResponseToChannel` Collision "ECC_Camera" NewResponse)))

(fn `UserConstructionScript`
  (`SceneComponent.SetHiddenInGame` (`self.TextRender`) (`self.HideText`) false)
  (`SceneComponent.SetHiddenInGame` (`self.InRange`) (`self.HideRange`) false))